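; BP_Intractable is an interactable actor that swaps between two meshes when interacted with.
; BeginPlay shows Mesh01 and hides Mesh02, and OnInteract reverses that visibility one way, with no path back.
; IsInteractable always returns false, independent of which mesh is showing.
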(event EventBeginPlay
  (Rendering|SetVisibility (Variables|Default|GetMesh01) true false)
  (Rendering|SetVisibility (Variables|Default|GetMesh02) false false))

(event EventOnInteract
  (params (LastPossess :type BP%20Frog%20Object%20Reference))
  (Rendering|SetVisibility (Variables|Default|GetMesh01) false false)
  (Rendering|SetVisibility (Variables|Default|GetMesh02) true false))

(fn ConstructionScript)

(fn IsInteractable
  (return false))