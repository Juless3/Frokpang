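; GM_Level is the gameplay level's game mode, handling startup UI, tutorial gating and end of game.
; BeginPlay sets game-only input, reads GI_Instance's tutorial flag to gate interaction and hitting, then adds the crosshair plus score or first-play tutorial widget.
; Tick pushes GMScore to the score widget.
; EndGame stores the score in GI_Instance, saves new highscores and opens L_Ende; NewHighscore is set false either way.
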(event Custom|EndGame
  (bind _gmscore (Variables|Default|GetGMScore))
  ;[0.3236 1 0.2872] EndGame
  (bind _asgi_instance (Utilities|Casting|CastToGI_Instance (Game|GetGameInstance))
    (:then
      (Variables|/Game/Blueprints/GI_Instance.GI_Instance_C|SetInstanceScore _asgi_instance _gmscore)
      (if (> _gmscore (Variables|/Game/Blueprints/BP_SaveGame.BP_SaveGame_C|GetInstanceHighscore (Variables|/Game/Blueprints/GI_Instance.GI_Instance_C|GetLoadedGame _asgi_instance)))
        (Variables|/Game/Blueprints/GI_Instance.GI_Instance_C|SetInstanceHighscore _asgi_instance (Variables|Default|GetGMScore))
        (Default|SetupSaveGame (Variables|Default|GetAs%20GI%20Instance))
        (Variables|/Game/Blueprints/GI_Instance.GI_Instance_C|SetNewHighscore _asgi_instance false)
        (else
          (Variables|/Game/Blueprints/GI_Instance.GI_Instance_C|SetNewHighscore _asgi_instance false)))
      (Game|OpenLevel(byName) "L_Ende"))
    (:CastFailed
      (Development|PrintString "GameModeLevelCastFailed"))))

(event Custom|ShowIngameUI
  ;[0.3236 1 0.2872] Comment
  ;;[1 1 1] Comment
  (bind _returnvalue (UserInterface|CreateWidget "/Game/Blueprints/UI/WBP_Score.WBP_Score_C"))
  (bind _output_get (Variables|Default|SetScoreWidget _returnvalue))
  (UserInterface|Viewport|AddtoViewport _output_get 0))

(event Custom|SetupInput
  (bind _returnvalue (Game|GetPlayerController 0))
  ;[0.3236 1 0.2872] Comment
  ;;[1 1 1] Comment
  (Input|SetInputModeGameOnly _returnvalue false)
  (Variables|/Script/Engine.PlayerController|SetbShowMouseCursor _returnvalue false))

(event Custom|CastToInstance
  ;[0.3236 1 0.2872] Comment
  ;;[1 1 1] Comment
  (bind _asgi_instance (Utilities|Casting|CastToGI_Instance (Game|GetGameInstance)))
  (bind _output_get (Variables|Default|SetAs%20GI%20Instance _asgi_instance))
  (if (Variables|/Game/Blueprints/GI_Instance.GI_Instance_C|GetTutorial _output_get)
    (Variables|Default|SetcanInteract false)
    (Variables|Default|SetcanHit false)
    (else
      (Variables|Default|SetcanInteract true)
      (Variables|Default|SetcanHit true))))

(event Custom|CheckForTutorial
  ;[0.3236 1 0.2872] Comment
  ;;[1 1 1] Comment
  (Variables|Default|SetGMtutorial (Variables|/Game/Blueprints/GI_Instance.GI_Instance_C|GetTutorial (Variables|Default|GetAs%20GI%20Instance))))

(event Custom|StartGame
  (if (Variables|Default|GetGMtutorial)
    (if (Variables|/Game/Blueprints/GI_Instance.GI_Instance_C|GetSchonmalGespielt (Variables|Default|GetAs%20GI%20Instance))
      (CallFunction|ShowIngameUI :!label _label)
      (else
        (CallFunction|ShowTutorial)))
    (else
      (goto _label))))

(event Custom|ShowTutorial
  (bind _returnvalue (UserInterface|CreateWidget "/Game/Blueprints/UI/WBP_TutorialText.WBP_TutorialText_C"))
  (UserInterface|Viewport|AddtoViewport _returnvalue 0))

(event EventBeginPlay
  (CallFunction|SetupInput)
  (CallFunction|CasttoInstance)
  (CallFunction|CheckforTutorial)
  (bind _returnvalue (UserInterface|CreateWidget "/Game/Blueprints/UI/WBP_Crosshair.WBP_Crosshair_C"))
  (UserInterface|Viewport|AddtoViewport _returnvalue 0)
  (CallFunction|StartGame))

(event EventTick
  (params (DeltaSeconds :type Float%20%28single-precision%29))
  ;[1 1 1] Tick
  (bind _scorewidget (Variables|Default|GetScoreWidget)
    (:then
      (Variables|/Game/Blueprints/UI/WBP_Score.WBP_Score_C|SetScore _scorewidget (Variables|Default|GetGMScore)))
    (:else)))

(fn ConstructionScript)