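; BP_Frog is the player-controlled frog, handling movement, camera look, interaction and pausing through Enhanced Input.
; It registers IMC_Frog on BeginPlay, moves relative to control yaw, and scales look by sensitivity with optional Y inversion.
; A Box overlap tracks one current BPI_Interact actor and toggles its highlight.
; The hit input sends that actor an OnHit interface message, and pause adds a new WBP_PauseMenu to the viewport.
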(event OnComponentEndOverlap(Box)
  (params (OverlappedComponent :type Primitive%20Component%20Object%20Reference) (OtherActor :type Actor%20Object%20Reference) (OtherComp :type Primitive%20Component%20Object%20Reference) (OtherBodyIndex :type Integer))
  ;[0.2779 0.6803 1] Set Current Interactable
  (if (Utilities|DoesObjectImplementInterface OtherActor "/Game/Blueprints/Interfaces/BPI_Interact.BPI_Interact_C")
    (Class|BPIInteract|SetHighlight(Message) OtherActor false)
    (Variables|Default|SetCurrentInteractable 0)))

(event OnComponentBeginOverlap(Box)
  (params (OverlappedComponent :type Primitive%20Component%20Object%20Reference) (OtherActor :type Actor%20Object%20Reference) (OtherComp :type Primitive%20Component%20Object%20Reference) (OtherBodyIndex :type Integer) (bFromSweep :type Boolean) (SweepResult :type Hit%20Result%20Structure%20%28by%20ref%29))
  ;[0.2779 0.6803 1] Set Current Interactable
  (if (Utilities|DoesObjectImplementInterface OtherActor "/Game/Blueprints/Interfaces/BPI_Interact.BPI_Interact_C")
    (bind _output_get (Variables|Default|SetCurrentInteractable OtherActor))
    (Class|BPIInteract|SetHighlight(Message) _output_get true)))

(event Custom|SetupInput
  ;[1 1 1] SetupInput
  (Input|AddMappingContext (PlayerController|LocalPlayerSubsystems|GetEnhancedInputLocalPlayerSubsystem (Game|GetPlayerController 0)) "/Game/Inputs/IMC_Frog.IMC_Frog" 0 "(bIgnoreAllPressedKeysUntilRelease=True,bForceImmediately=False,bNotifyUserSettings=False)"))

(event EventBeginPlay
  (CallFunction|SetupInput))

(event Input|EnhancedActionEvents|EnhancedInputActionIA_Pause
  (params (ActionValue :type Boolean) (ElapsedSeconds :type Float%20%28double-precision%29) (TriggeredSeconds :type Float%20%28double-precision%29) (InputAction :type Input%20Action%20Object%20Reference :default "/Game/Inputs/IA_Pause.IA_Pause"))
  (:Started
    (bind _returnvalue (UserInterface|CreateWidget "/Game/Blueprints/UI/WBP_PauseMenu.WBP_PauseMenu_C"))
    (UserInterface|Viewport|AddtoViewport _returnvalue 0)))

(event Input|EnhancedActionEvents|EnhancedInputActionIA_Move
  (params (ActionValue :type Vector%202D%20Structure) (ElapsedSeconds :type Float%20%28double-precision%29) (TriggeredSeconds :type Float%20%28double-precision%29) (InputAction :type Input%20Action%20Object%20Reference :default "/Game/Inputs/IA_Move.IA_Move"))
  ;[1 1 1] Move
  (Pawn|Input|AddMovementInput (Math|Vector|GetForwardVector (Math|Rotator|MakeRotator 0.0 0.0 (.yaw (Pawn|GetControlRotation :!class /Script/Engine.Pawn)))) (.y ActionValue) false)
  (Pawn|Input|AddMovementInput (Math|Vector|GetRightVector (Math|Rotator|MakeRotator 0.0 0.0 (.yaw (Pawn|GetControlRotation :!class /Script/Engine.Pawn)))) (.x ActionValue) false))

(event Input|EnhancedActionEvents|EnhancedInputActionIA_Look
  (params (ActionValue :type Vector%202D%20Structure) (ElapsedSeconds :type Float%20%28double-precision%29) (TriggeredSeconds :type Float%20%28double-precision%29) (InputAction :type Input%20Action%20Object%20Reference :default "/Game/Inputs/IA_Look.IA_Look"))
  ;[1 1 1] Look
  (Pawn|Input|AddControllerYawInput (* (.x ActionValue) (Variables|Default|GetRotateSensitivity)))
  (Pawn|Input|AddControllerPitchInput (* (.y ActionValue) (Variables|Default|GetRotateSensitivity) (Math|Integer|SelectInt 1 -1 (Variables|Default|GetInvertYaxis)))))

(event Input|EnhancedActionEvents|EnhancedInputActionIA_Hit
  (params (ActionValue :type Boolean) (ElapsedSeconds :type Float%20%28double-precision%29) (TriggeredSeconds :type Float%20%28double-precision%29) (InputAction :type Input%20Action%20Object%20Reference :default "/Game/Inputs/IA_Hit.IA_Hit"))
  ;[1 1 1] Interact
  (:Started
    (bind _currentinteractable (Variables|Default|GetCurrentInteractable)
      (:then
        (Class|BPIInteract|OnHit(Message) _currentinteractable self))
      (:else))))

(fn ConstructionScript)