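; Interactable, hittable microwave that plays a click sound and starts smoking when used.
; The first use spawns Niagara smoke, sets a clicked flag on the level game mode, and shows a tutorial widget if the game has not been played before.
; BeginPlay reads that flag to restore smoke on an already clicked microwave.
; Hits stop the sound and hide interaction-spawned smoke; the smoke restored at BeginPlay is not stored, so it stays visible.
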(event EventBeginPlay
  (|CallParentFunction)
  (bind _asgm_level (Utilities|Casting|CastToGM_Level (Game|GetGameMode)))
  (bind _output_get (Variables|Default|SetGameMdoe _asgm_level))
  (if (Variables|/Game/Blueprints/GM_Level.GM_Level_C|GetMicrowaveclicked _output_get)
    (AddComponent|AddNiagaraComponent false (Math|Transform|MakeTransform (Variables|/Script/Engine.SceneComponent|GetRelativeLocation (Variables|Default|GetSmokeLocation)) "0, 0, 0" "1.000000,1.000000,1.000000"))
    (else
      (Variables|Default|SetNoNo true))))

(event Collision|EventActorBeginOverlap
  (params (OtherActor :type Actor%20Object%20Reference)))

(event EventTick
  (params (DeltaSeconds :type Float%20%28single-precision%29)))

(event EventOnInteract
  (params (LastPossess :type BP%20Frog%20Object%20Reference))
  (bind _returnvalue (Audio|SpawnSound2D "/Game/Sounds/Interactions/MS_MicrowelleCLick.MS_MicrowelleCLick" 1.0 1.0 0.0 0))
  (Variables|Default|SetSound _returnvalue)
  (if (Variables|Default|GetNoNo)
    (Utilities|FlowControl|DoOnce false
      (:Completed
        (bind _returnvalue_2 (AddComponent|AddNiagaraComponent false (Math|Transform|MakeTransform (Variables|/Script/Engine.SceneComponent|GetRelativeLocation (Variables|Default|GetSmokeLocation)) "0, 0, 0" "1.000000,1.000000,1.000000")))
        (Variables|Default|SetNiagara _returnvalue_2)
        (Variables|/Game/Blueprints/GM_Level.GM_Level_C|SetMicrowaveclicked (Variables|Default|GetGameMdoe) true)
        (if (not (Variables|/Game/Blueprints/GI_Instance.GI_Instance_C|GetSchonmalGespielt (Variables|Default|GetGameInstanceVariable)))
          (bind _returnvalue_3 (UserInterface|CreateWidget "/Game/Blueprints/UI/WBP_TutorialText02.WBP_TutorialText02_C"))
          (UserInterface|Viewport|AddtoViewport _returnvalue_3 0))))))

(event EventOnHit
  (params (LastPossess :type BP%20Frog%20Object%20Reference))
  (bind _sound (Variables|Default|GetSound))
  (bind _niagara (Variables|Default|GetNiagara))
  (|CallParentFunction 0)
  (Utilities|IsValid _sound
    (:Is%20Valid
      (Audio|Components|Audio|Stop _sound))
    (:Is%20Not%20Valid
      _))
  (Utilities|IsValid _niagara
    (:Is%20Valid
      (Rendering|SetVisibility _niagara false false))))

(fn ConstructionScript
  (|CallParentFunction))