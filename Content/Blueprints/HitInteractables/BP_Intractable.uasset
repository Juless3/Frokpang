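; BP_Intractable is a breakable interactable that scores a point when hit and supports an overlay-material highlight.
; Breaking plays a sound and Niagara puff, reveals Mesh02, then destroys Mesh01, its children and the Box.
; Unless the game instance's SchonmalGespielt ("already played") flag is set, game mode flags require the microwave to be clicked, then destroyed before other objects can break.
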(event Custom|Test
  (Development|PrintString "Interacted"))

(event EventBeginPlay
  (Rendering|SetVisibility (Variables|Default|GetMesh01) true true)
  (Rendering|SetVisibility (Variables|Default|GetMesh02) false true)
  (bind _asgm_level (Utilities|Casting|CastToGM_Level (Game|GetGameMode)))
  (Variables|Default|SetGameModeVariable _asgm_level)
  (bind _asgi_instance (Utilities|Casting|CastToGI_Instance (Game|GetGameInstance)))
  (Variables|Default|SetGameInstanceVariable _asgi_instance))

(event EventSetHighlight
  (params (On :type Boolean))
  (if On
    (bind _mesh01 (Variables|Default|GetMesh01)
      (:then
        (Rendering|Material|SetOverlayMaterial _mesh01 "/Game/Materials/Overlays/M_OverlayBaseMat.M_OverlayBaseMat" :!class /Script/Engine.MeshComponent))
      (:else))
    (else
      (bind _mesh01_2 (Variables|Default|GetMesh01)
        (:then
          (Rendering|Material|SetOverlayMaterial _mesh01_2 0 :!class /Script/Engine.MeshComponent))
        (:else)))))

(event EventOnHit
  (params (LastPossess :type BP%20Frog%20Object%20Reference))
  (if (Variables|/Game/Blueprints/GI_Instance.GI_Instance_C|GetSchonmalGespielt (Variables|Default|GetGameInstanceVariable))
    (Audio|SpawnSound2D "/Game/Sounds/Interactions/MS_Kaputt.MS_Kaputt" 1.0 1.0 0.0 0 :!label _label)
    (bind _returnvalue (AddComponent|AddNiagaraComponent false (Math|Transform|MakeTransform (Variables|/Script/Engine.SceneComponent|GetRelativeLocation (Variables|Default|GetPUFFLOCATION)) "0, 0, 0" "1.000000,1.000000,1.000000")))
    (Components|Activation|Activate _returnvalue false)
    (Rendering|SetVisibility (Variables|Default|GetMesh02) true true)
    (Math|Integer|IncrementInt (Variables|/Game/Blueprints/GM_Level.GM_Level_C|GetGMScore (Variables|Default|GetGameModeVariable))
      (:%20%20
        (bind _mesh01 (Variables|Default|GetMesh01)
          (:then
            (bind _output_get (Variables|Default|SetLength (Utilities|Array|Length (Components|GetChildrenComponents _mesh01 true))))
            (for _index (range 0 _output_get)
              (Utilities|IsValid (Utilities|Array|Get(acopy) (Components|GetChildrenComponents _mesh01 true))
                (:Is%20Valid
                  (Components|DestroyComponent (Utilities|Array|Get(acopy) (Components|GetChildrenComponents _mesh01 true))))))
            (Utilities|FlowControl|Delay 0.025)
            (Components|DestroyComponent _mesh01))
          (:else
            _))
        (Utilities|FlowControl|Delay 0.025)
        (bind _box (Variables|Default|GetBox)
          (:then
            (Components|DestroyComponent _box))
          (:else
            _))
        (Components|Activation|Deactivate _returnvalue)))
    (elif (Variables|/Game/Blueprints/GM_Level.GM_Level_C|GetMicrowaveclicked (Variables|Default|GetGameModeVariable))
      (if (Variables|Default|GetMicrowave?)
        (Variables|/Game/Blueprints/GM_Level.GM_Level_C|SetMicrowavedestroyed (Variables|Default|GetGameModeVariable) true)
        (goto _label)
        (elif (Variables|/Game/Blueprints/GM_Level.GM_Level_C|GetMicrowavedestroyed (Variables|Default|GetGameModeVariable))
          (goto _label))))))

(fn ConstructionScript)

(fn IsInteractable
  (return (Variables|Default|GetInteractable)))