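; Game instance that owns the save game holding volume levels, frame rate limit, graphics quality and high score.
; On Init it loads or creates the BP_SaveGame, then applies its master, music and sound volumes through sound mix overrides a tick later.
; FPS and graphics values are read from GameUserSettings rather than the save.
; SetupSaveGame copies the instance's own variables into the save and writes the slot; loading does not copy saved values back into them.
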(event Custom|initVolume
  (bind _loadedgame (Variables|Default|GetLoadedGame))
  (Utilities|FlowControl|DelayUntilNextTick)
  (Audio|SetSoundMixClassOverride "/Game/Sounds/Settings/SC_SoundClassMixer.SC_SoundClassMixer" "/Game/Sounds/Settings/SC_Master.SC_Master" (Variables|/Game/Blueprints/BP_SaveGame.BP_SaveGame_C|GetMasterVolume _loadedgame) 1.0 0.0 true)
  (Audio|SetSoundMixClassOverride "/Game/Sounds/Settings/SC_SoundClassMixer.SC_SoundClassMixer" "/Game/Sounds/Settings/SC_Music.SC_Music" (Variables|/Game/Blueprints/BP_SaveGame.BP_SaveGame_C|GetMusicVolume _loadedgame) 1.0 0.0 true)
  (Audio|SetSoundMixClassOverride "/Game/Sounds/Settings/SC_SoundClassMixer.SC_SoundClassMixer" "/Game/Sounds/Settings/SC_Sound.SC_Sound" (Variables|/Game/Blueprints/BP_SaveGame.BP_SaveGame_C|GetSoundVolume _loadedgame) 1.0 0.0 true))

(event Custom|SetupLoadGame
  (bind _returnvalue (SaveGame|DoesSaveGameExist (Variables|Default|GetSaveSlot)))
  (if _returnvalue
    (bind _returnvalue_2 (SaveGame|LoadGamefromSlot (Variables|Default|GetSaveSlot)))
    (Development|PrintString (Utilities|String|Append (Utilities|GetDisplayName _returnvalue_2) "ASDF"))
    (bind _asbp_save_game (Utilities|Casting|CastToBP_SaveGame _returnvalue_2))
    (Variables|Default|SetLoadedGame _asbp_save_game)
    (bind _returnvalue_3 (Settings|GetGameUserSettings))
    (Variables|Default|SetFPS (Class|GameUserSettings|GetFrameRateLimit _returnvalue_3))
    (bind _returnvalue_4 (Settings|GetGameUserSettings))
    (Variables|Default|SetGraphic (Class|GameUserSettings|GetOverallScalabilityLevel _returnvalue_4))
    (Development|PrintString (Utilities|String|ToString(Integer) (Variables|/Game/Blueprints/BP_SaveGame.BP_SaveGame_C|GetInstanceHighscore (Variables|Default|GetLoadedGame))))
    (else
      (bind _returnvalue_5 (SaveGame|CreateSaveGameObject "/Game/Blueprints/BP_SaveGame.BP_SaveGame_C"))
      (bind _asbp_save_game_2 (Utilities|Casting|CastToBP_SaveGame _returnvalue_5))
      (Variables|Default|SetLoadedGame _asbp_save_game_2)
      (bind _returnvalue_6 (Settings|GetGameUserSettings))
      (Variables|Default|SetFPS (Class|GameUserSettings|GetFrameRateLimit _returnvalue_6))
      (bind _returnvalue_7 (Settings|GetGameUserSettings))
      (Variables|Default|SetGraphic (Class|GameUserSettings|GetOverallScalabilityLevel _returnvalue_7))
      (Development|PrintString (Utilities|String|ToString(Integer) (Variables|/Game/Blueprints/BP_SaveGame.BP_SaveGame_C|GetInstanceHighscore (Variables|Default|GetLoadedGame)))))))

(event Custom|SetupSaveGame
  (Variables|/Game/Blueprints/BP_SaveGame.BP_SaveGame_C|SetMasterVolume (Variables|Default|GetLoadedGame) (Variables|Default|GetMasterVolume))
  (Variables|/Game/Blueprints/BP_SaveGame.BP_SaveGame_C|SetMusicVolume (Variables|Default|GetLoadedGame) (Variables|Default|GetMusicVolume))
  (Variables|/Game/Blueprints/BP_SaveGame.BP_SaveGame_C|SetSoundVolume (Variables|Default|GetLoadedGame) (Variables|Default|GetSoundVolume))
  (Variables|/Game/Blueprints/BP_SaveGame.BP_SaveGame_C|SetFPS (Variables|Default|GetLoadedGame) (Variables|Default|GetFPS))
  (Variables|/Game/Blueprints/BP_SaveGame.BP_SaveGame_C|SetGraphic (Variables|Default|GetLoadedGame) (Variables|Default|GetGraphic))
  (Variables|/Game/Blueprints/BP_SaveGame.BP_SaveGame_C|SetInstanceHighscore (Variables|Default|GetLoadedGame) (Variables|Default|GetInstanceHighscore))
  (SaveGame|SaveGametoSlot (Variables|Default|GetLoadedGame) (Variables|Default|GetSaveSlot)))

(event EventInit
  (CallFunction|SetupLoadGame)
  (CallFunction|InitVolume)
  (bind _returnvalue (Settings|GetGameUserSettings))
  (Variables|Default|SetFPS (Class|GameUserSettings|GetFrameRateLimit _returnvalue))
  (bind _returnvalue_2 (Settings|GetGameUserSettings))
  (Variables|Default|SetGraphic (Class|GameUserSettings|GetOverallScalabilityLevel _returnvalue_2)))